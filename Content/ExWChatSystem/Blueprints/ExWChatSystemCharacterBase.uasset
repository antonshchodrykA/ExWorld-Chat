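; Test character Blueprint for the ExW chat system, connecting a player to the main chat UI and an overhead-style bubble widget.
; On BeginPlay the locally controlled character picks a random test name, sends it to the server and creates the chat widget.
; Enter switches to UI-only input with cursor; number keys randomize zone, race, party or guild.
; Events push updated values to the chat UI and messages to the bubble.
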(event `self.ReceiveBeginPlay`
  (if (`self.IsLocallyControlled`)
    (bind _output_get (set `self.PlayerName` (`self.GetTestRandomPlayerName`)))
    (`self.ServerSetPlayerName` _output_get)
    (bind _returnvalue (`|CreateWidget` "/Game/ExWChatSystem/Blueprints/UMG/UMG_ExWChatSystemMain.UMG_ExWChatSystemMain_C" null (`self.PlayerName`)))
    (`UserWidget.AddToViewport` _returnvalue 0)
    (set `self.ChatUserWidget` _returnvalue)
    (set `self.BP_ChatUserWidget` _returnvalue)))

(event `Key|Enter`
  (params (Key :type "Key Structure"))
  (:`Pressed`
    (`WidgetBlueprintLibrary.SetInputMode_UIOnlyEx` (`GameplayStatics.GetPlayerController` 0) null)
    (set `PlayerController.bShowMouseCursor` true (`GameplayStatics.GetPlayerController` 0))))

(event `self.OnTestCharacterValuesUpdated`
  (`/Game/ExWChatSystem/Blueprints/UMG/UMG_ExWChatSystemMain.UpdateTestCharacterProperties` (`self.BP_ChatUserWidget`) (`self.MacroZone`) (`self.Race`) (`self.Party`) (`self.Guild`)))

(event `Key|One`
  (params (Key :type "Key Structure"))
  (:`Pressed`
    (`self.SetRandomMacroZone`)))

(event `Key|Two`
  (params (Key :type "Key Structure"))
  (:`Pressed`
    (`self.SetRandomRace`)))

(event `Key|Three`
  (params (Key :type "Key Structure"))
  (:`Pressed`
    (`self.SetRandomParty`)))

(event `Key|Four`
  (params (Key :type "Key Structure"))
  (:`Pressed`
    (`self.SetRandomGuild`)))

(event `self.OnShowMessageInBubble`
  (params (Message :type String))
  (`/Game/ExWChatSystem/Blueprints/UMG/UMG_ExWChatSystemBubble.ShowMessage` (cast `/Game/ExWChatSystem/Blueprints/UMG/UMG_ExWChatSystemBubble` (`WidgetComponent.GetUserWidgetObject` (`self.BubbleChat`)) :!pure true) Message))

(fn `GetTestRandomPlayerName`
  (returns (Output :type String))
  (bind _array (`|MakeArray` "Carlos" "Pepe" "Arturo" "Gaby"))
  (return (`|GetArrayItem` _array (`KismetMathLibrary.RandomIntegerInRange` 0 (- (`KismetArrayLibrary.Array_Length` _array) 1)))))

(fn `UserConstructionScript`)